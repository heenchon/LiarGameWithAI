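; BP_PC_Chat is a player controller that handles player text chat.
; On BeginPlay the local controller creates and displays a WBP_ChatPanel widget, and pressing Enter gives its ChatScroll keyboard focus.
; SR_SubmitChat loops through the GameState's PlayerArray and relays the name and message to each chat controller's OC_UpdateChat, which updates that controller's panel.
; The SR and OC prefixes suggest a server-to-owning-client RPC pattern.
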(event `self.ReceiveBeginPlay`
  (if (`self.IsLocalPlayerController`)
    (bind _returnvalue (`|CreateWidget` "/Game/ChatUI/WBP_ChatPanel.WBP_ChatPanel_C" self))
    (bind _output_get (set `self.WBP_ChatPanel` _returnvalue))
    (`UserWidget.AddToViewport` _output_get 0)))

(event `Key|Enter`
  (params (Key :type "Key Structure"))
  (:`Pressed`
    (bind _wbp_chatpanel (`self.WBP_ChatPanel`)
      (:`then`
        (`Widget.SetKeyboardFocus` (`/Game/ChatUI/WBP_ChatPanel.ChatScroll` _wbp_chatpanel)))
      (:`else`))))

(event `SR_SubmitChat`
  (params (PlayerName :type Text) (Chat :type Text))
  (for _array_element (`GameStateBase.PlayerArray` (`GameplayStatics.GetGameState`))
    (bind _asbp_pc_chat (cast `/Game/ChatUI/BP_PC_Chat` (`PlayerState.GetPlayerController` _array_element)))
    (`self.OC_UpdateChat` _asbp_pc_chat PlayerName Chat)))

(event `OC_UpdateChat`
  (params (PlayerName :type Text) (Chat :type Text))
  (bind _wbp_chatpanel (`self.WBP_ChatPanel`)
    (:`then`
      (`/Game/ChatUI/WBP_ChatPanel.UpdateChat` _wbp_chatpanel PlayerName Chat))
    (:`else`)))

(fn `UserConstructionScript`)